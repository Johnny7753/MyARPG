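; JumpSectionNS is an anim notify state that marks a combo window within the player character's animation.
; On begin, it sets EnableComboPeriod on the owning BP_PlayerCharacter and registers itself as that character's JumpSectionNotify.
; On end, it disables the combo period and clears the reference, so the notify's span defines when combo input is allowed.
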(fn ReceivedNotifyBegin
  (params (MeshComp :type Skeletal%20Mesh%20Component%20Object%20Reference) (Animation :type Anim%20Sequence%20Base%20Object%20Reference) (TotalDuration :type Float%20%28single-precision%29) (EventReference :type Anim%20Notify%20Event%20Reference%20Structure%20%28by%20ref%29))
  (bind _asbp_player_character (Utilities|Casting|CastToBP_PlayerCharacter (Components|GetOwner MeshComp)))
  (Variables|/Game/Blueprint/Character/BP_PlayerCharacter.BP_PlayerCharacter_C|SetbEnableComboPeriod _asbp_player_character true)
  (Variables|/Game/Blueprint/Character/BP_PlayerCharacter.BP_PlayerCharacter_C|SetJumpSectionNotify _asbp_player_character self)
  (return false))

(fn ReceivedNotifyEnd
  (params (MeshComp :type Skeletal%20Mesh%20Component%20Object%20Reference) (Animation :type Anim%20Sequence%20Base%20Object%20Reference) (EventReference :type Anim%20Notify%20Event%20Reference%20Structure%20%28by%20ref%29))
  (bind _asbp_player_character (Utilities|Casting|CastToBP_PlayerCharacter (Components|GetOwner MeshComp)))
  (Variables|/Game/Blueprint/Character/BP_PlayerCharacter.BP_PlayerCharacter_C|SetbEnableComboPeriod _asbp_player_character false)
  (Variables|/Game/Blueprint/Character/BP_PlayerCharacter.BP_PlayerCharacter_C|SetJumpSectionNotify _asbp_player_character 0)
  (return false))