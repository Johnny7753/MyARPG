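; Goblin NPC character Blueprint that sets up a weapon-wielding goblin when play begins.
; After the parent BeginPlay, it stores its mesh, creates a weapon from the weapon class, attaches it at a named socket and selects the hammer attack montage.
; The construction script only calls the parent, and the overlap and tick events are disabled stubs.
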(event EventBeginPlay
  (|CallParentFunction)
  (Variables|Default|SetThisMesh (Variables|Character|GetMesh))
  (CallFunction|CreateWeapon (Variables|Default|GetWeaponClass))
  (CallFunction|AttachWeapon (Variables|Default|GetSocket%20Name))
  (Variables|Default|SetMontage "/Game/Characters/Animations/AM_Attack_Hammer.AM_Attack_Hammer"))

(event Collision|EventActorBeginOverlap
  (params (OtherActor :type Actor%20Object%20Reference))
  (|CallParentFunction OtherActor) ; This node is disabled and will not be called.\nDrag off pins to build functionality.
)

(event EventTick
  (params (DeltaSeconds :type Float%20%28single-precision%29))
  (|CallParentFunction DeltaSeconds) ; This node is disabled and will not be called.\nDrag off pins to build functionality.
)

(fn ConstructionScript
  (|CallParentFunction))