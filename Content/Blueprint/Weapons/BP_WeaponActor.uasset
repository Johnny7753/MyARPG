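; BP_WeaponActor is a weapon actor that deals melee-style damage to actors it overlaps during an attack.
; BeginWeaponAttack and EndWeaponAttack toggle the attack window, with the former also setting the damage amount.
; Overlaps skip actors of the instigator's class and pass a DoOnce that resets shortly after overlap ends, limiting repeat hits.
; Damage credits player controller zero, then calls HitPause, which is an empty stub.
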(event EventBeginPlay)

(event Collision|EventActorBeginOverlap
  (params (OtherActor :type Actor%20Object%20Reference))
  (if (and (!= (Utilities|GetClass OtherActor) (Utilities|GetClass (Game|GetInstigator))) (Variables|Default|GetIsAttacking))
    (Utilities|FlowControl|DoOnce false
      (:Completed
        (Game|Damage|ApplyDamage OtherActor (Variables|Config|GetBase%20Damage) (Game|GetPlayerController 0) self)
        (CallFunction|HitPause)))))

(event EventTick
  (params (DeltaSeconds :type Float%20%28single-precision%29)))

(event Collision|EventActorEndOverlap
  (params (OtherActor :type Actor%20Object%20Reference))
  (Utilities|FlowControl|Delay 0.2)
  (Utilities|FlowControl|DoOnce false) ; enters at Reset
)

(fn ConstructionScript)

(fn HitPause)

(fn BeginWeaponAttack
  (params (WeaponDamage :type Float%20%28double-precision%29))
  (Variables|Default|SetIsAttacking true)
  (Variables|Config|SetBase%20Damage WeaponDamage))

(fn EndWeaponAttack
  (Variables|Default|SetIsAttacking false))